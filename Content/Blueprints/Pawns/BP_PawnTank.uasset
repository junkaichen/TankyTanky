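; Player tank pawn Blueprint that manages the HUD, pause menu and saved progress.
; BeginPlay loads level stage and total score from the save slot, or creates a new save, then creates the HUD.
; A looping timer counts down MovieTime, then clears all widgets and shows the HUD.
; Tick drives health, ammo and remaining-tower displays through dynamic material parameters, with ammo bar divisions depending on magazine size.
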(event `self.ReceiveBeginPlay`
  (`KismetSystemLibrary.K2_SetTimer` null "MovieTime" 1.0 true)
  (bind _returnvalue (`GameplayStatics.DoesSaveGameExist` (`self.SaveSlot`)))
  (if _returnvalue
    (`self.LoadGame`)
    (bind _returnvalue_2 (`|CreateWidget` "/Game/Blueprints/Widgets/WBP_HUD.WBP_HUD_C"))
    (set `self.HUD_REF` _returnvalue_2)
    (else
      (bind _returnvalue_3 (`GameplayStatics.CreateSaveGameObject` "/Game/BP__MySaveGame.BP__MySaveGame_C"))
      (bind _asbp__my_save_game (cast `/Game/BP__MySaveGame` _returnvalue_3))
      (set `self.SavedGameReference` _asbp__my_save_game)
      (`self.SaveGame`)
      (bind _returnvalue_4 (`|CreateWidget` "/Game/Blueprints/Widgets/WBP_HUD.WBP_HUD_C"))
      (set `self.HUD_REF` _returnvalue_4))))

(event `self.ReceiveTick`
  (params (DeltaSeconds :type "Float (single-precision)"))
  (`self.Update Ammo HUD`)
  (`self.Update Health Bar`)
  (`self.Update EnemyNumber`))

(event `Key|E`
  (params (Key :type "Key Structure")))

(event `Key|B`
  (params (Key :type "Key Structure")))

(event `InputAction|PauseGame` :paused true
  (params (Key :type "Key Structure"))
  (bind _returnvalue (`GameplayStatics.GetPlayerController` 0))
  (bind _pausemenuref (`self.PauseMenuREF`))
  ;[1 1 1] Pause/-UnPause Game
  (:`Pressed`
    (`/Engine/EditorBlueprintResources/StandardMacros.IsValid` (`self.PauseMenuREF`)
      (:`Is Valid`
        _)
      (:`Is Not Valid`
        (bind _returnvalue_2 (`|CreateWidget` "/Game/Blueprints/Widgets/WBP_PauseMenu.WBP_PauseMenu_C"))
        (set `self.PauseMenuREF` _returnvalue_2)))
    (if (`GameplayStatics.IsGamePaused`)
      (`Widget.RemoveFromParent` _pausemenuref)
      (`GameplayStatics.SetGamePaused` false)
      (else
        (`UserWidget.AddToViewport` _pausemenuref 0)
        (`GameplayStatics.SetGamePaused` true)
        (set `PlayerController.bShowMouseCursor` true _returnvalue)
        (`WidgetBlueprintLibrary.SetInputMode_GameAndUIEx` _returnvalue _pausemenuref "LockInFullscreen" false)))))

(fn `LoadAndSetSavedVariables`
  (bind _savedgamereference (`self.SavedGameReference`))
  ;[1 1 1] Set the Variable for Character
  (bind _asbp_pawn_tank (cast `/Game/Blueprints/Pawns/BP_PawnTank` (`GameplayStatics.GetPlayerPawn` 0)))
  (set `Tank.LevelStage` (`/Game/BP__MySaveGame.LevelStageSaved` _savedgamereference) _asbp_pawn_tank)
  (set `self.TotalPoints` (`/Game/BP__MySaveGame.PlayerTotalScoreSaved` _savedgamereference)))

(fn `LoadGame`
  (bind _returnvalue (`GameplayStatics.LoadGameFromSlot` (`self.SaveSlot`)))
  (bind _asbp__my_save_game (cast `/Game/BP__MySaveGame` _returnvalue))
  (set `self.SavedGameReference` _asbp__my_save_game)
  (`self.LoadAndSetSavedVariables`))

(fn `MovieTime`
  (set `self.Movie_time` (- (`self.Movie_time`) 1))
  (if (<= (`self.Movie_time`) 0)
    (`WidgetLayoutLibrary.RemoveAllWidgets`)
    (`UserWidget.AddToViewport` (`self.HUD_REF`) 0)
    (`KismetSystemLibrary.K2_PauseTimer` null "MovieTime")))

(fn `SaveGame`
  (bind _savedgamereference (`self.SavedGameReference`))
  ;[1 1 1] Get the Variables that We want to Save
  (bind _asbp_pawn_tank (cast `/Game/Blueprints/Pawns/BP_PawnTank` (`GameplayStatics.GetPlayerPawn` 0)))
  ;[1 1 1] Set Them into the Save Game Object
  (set `/Game/BP__MySaveGame.PlayerTotalScoreSaved` (`Tank.TotalPoints` _asbp_pawn_tank) _savedgamereference)
  (set `/Game/BP__MySaveGame.LevelStageSaved` (`Tank.LevelStage` _asbp_pawn_tank) _savedgamereference)
  ;[1 1 1] Save the Save Game Object to Slot
  (bind _returnvalue (`GameplayStatics.SaveGameToSlot` (`self.SavedGameReference`) (`self.SaveSlot`)))
  (`KismetSystemLibrary.PrintString` (`KismetMathLibrary.SelectString` "Successful Saved" "Failed" _returnvalue))
  (`KismetSystemLibrary.PrintString` (`KismetStringLibrary.Conv_IntToString` (`/Game/BP__MySaveGame.LevelStageSaved` (`self.SavedGameReference`)))))

(fn `Update Ammo HUD`
  (if (`KismetSystemLibrary.IsValid` (`self.HUD_REF`))
    (`/Engine/EditorBlueprintResources/StandardMacros.CompareInt` (`self.FullAmmo`) 30
      (:`>`
        (bind _returnvalue (`Image.GetDynamicMaterial` (`/Game/Blueprints/Widgets/WBP_HUD.Ammo_Image` (`self.HUD_REF`))))
        (`MaterialInstanceDynamic.SetScalarParameterValue` _returnvalue "DivisionsCount" 1.0))
      (:`<`
        (bind _returnvalue_2 (`Image.GetDynamicMaterial` (`/Game/Blueprints/Widgets/WBP_HUD.Ammo_Image` (`self.HUD_REF`))))
        (`MaterialInstanceDynamic.SetScalarParameterValue` _returnvalue_2 "DivisionsCount" (`KismetMathLibrary.Conv_IntToDouble` (`self.FullAmmo`)))))
    (bind _returnvalue_3 (`Image.GetDynamicMaterial` (`/Game/Blueprints/Widgets/WBP_HUD.Ammo_Image` (`self.HUD_REF`))))
    (`MaterialInstanceDynamic.SetScalarParameterValue` _returnvalue_3 "Progress" (/ (`KismetMathLibrary.Conv_IntToDouble` (`self.Ammo`)) (`self.FullAmmo`)))))

(fn `Update EnemyNumber`
  (bind _asbp_toon_tank_game_mode (cast `/Game/Blueprints/GameMode/BP_ToonTankGameMode` (`GameplayStatics.GetGameMode`)))
  (if (`KismetSystemLibrary.IsValid` (`self.HUD_REF`))
    (bind _returnvalue (`Image.GetDynamicMaterial` (`/Game/Blueprints/Widgets/WBP_HUD.TargetImage` (`self.HUD_REF`))))
    (`MaterialInstanceDynamic.SetScalarParameterValue` _returnvalue "Progress" (/ (`KismetMathLibrary.Conv_IntToDouble` (`TookTanksGameMode.TargetTowers` _asbp_toon_tank_game_mode)) 20.0))))

(fn `Update Health Bar`
  (if (`KismetSystemLibrary.IsValid` (`self.HUD_REF`))
    (bind _returnvalue (`Image.GetDynamicMaterial` (`/Game/Blueprints/Widgets/WBP_HUD.Health_Image` (`self.HUD_REF`))))
    (`MaterialInstanceDynamic.SetScalarParameterValue` _returnvalue "Progress" (* (`HealthComponent.Health` (`self.Health`)) 0.01))))

(fn `UserConstructionScript`)