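; Tank game mode that handles the start screen, level completion and defeat.
; StartGame clears widgets, then shows the start widget and plays music.
; GameOver parses the level number from the level name, showing a final-pass widget for level 6.
; Other results show win or lose widgets and pause; winning the current stage also advances LevelStage on the pawn, updates the game instance and saves.
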(event `self.StartGame`
  (`WidgetLayoutLibrary.RemoveAllWidgets`)
  (bind _returnvalue (`|CreateWidget` "/Game/Blueprints/Widgets/WBP_StartGameWidget.WBP_StartGameWidget_C"))
  (`UserWidget.AddToViewport` _returnvalue 0)
  (`GameplayStatics.SpawnSound2D` "/Game/Assets/Audio/12-快乐嬉戏_12-Jolly-Frolic__爱给网_aigei_com.12-快乐嬉戏_12-Jolly-Frolic__爱给网_aigei_com" 1.0 1.0 0.0 null))

(event `self.ReceiveTick`
  (params (DeltaSeconds :type "Float (single-precision)")))

(event `self.GameOver`
  (params (bWonGame :type Boolean))
  (if bWonGame
    (bind _returnvalue (`GameplayStatics.GetCurrentLevelName` true))
    (bind _returnvalue_2 (`KismetStringLibrary.Conv_StringToInt` (`KismetStringLibrary.GetSubstring` _returnvalue 6)))
    (if (== _returnvalue_2 6)
      (`GameplayStatics.PlaySound2D` "/Game/Assets/Audio/过关.过关" 1.0 1.0 0.0 null null)
      (bind _returnvalue_3 (`|CreateWidget` "/Game/Blueprints/Widgets/WBP_FinalPass.WBP_FinalPass_C"))
      (`UserWidget.AddToViewport` _returnvalue_3 0)
      (else
        (bind _asbp_pawn_tank (cast `/Game/Blueprints/Pawns/BP_PawnTank` (`GameplayStatics.GetPlayerPawn` 0)))
        (if (== _returnvalue_2 (`Tank.LevelStage` _asbp_pawn_tank))
          (bind _returnvalue_4 (+ (`Tank.LevelStage` _asbp_pawn_tank) 1))
          (set `Tank.LevelStage` _returnvalue_4 _asbp_pawn_tank)
          (bind _asstore_vars_1 (cast `/Game/Blueprints/Store_Vars1` (`GameplayStatics.GetGameInstance`)))
          (set `/Game/Blueprints/Store_Vars1.LevelStageInstance` _returnvalue_4 _asstore_vars_1)
          (`/Game/Blueprints/Pawns/BP_PawnTank.SaveGame` _asbp_pawn_tank)
          (bind _returnvalue_5 (`|CreateWidget` "/Game/Blueprints/Widgets/WBP_EndGameWidget.WBP_EndGameWidget_C"))
          (`UserWidget.AddToViewport` _returnvalue_5 0)
          (`GameplayStatics.SetGamePaused` true)
          (`GameplayStatics.PlaySound2D` "/Game/Assets/Audio/过关.过关" 1.0 1.0 0.0 null null)
          (else
            (bind _returnvalue_6 (`|CreateWidget` "/Game/Blueprints/Widgets/WBP_EndGameWidget.WBP_EndGameWidget_C"))
            (`UserWidget.AddToViewport` _returnvalue_6 0)
            (`GameplayStatics.SetGamePaused` true)
            (`GameplayStatics.PlaySound2D` "/Game/Assets/Audio/过关.过关" 1.0 1.0 0.0 null null)))))
    (else
      (bind _returnvalue_7 (`|CreateWidget` "/Game/Blueprints/Widgets/WBP_LoseGameWidget.WBP_LoseGameWidget_C"))
      (`UserWidget.AddToViewport` _returnvalue_7 0)
      (`GameplayStatics.SetGamePaused` true)
      (`GameplayStatics.PlaySound2D` "/Game/Assets/Audio/失败.失败" 1.0 1.0 0.0 null null))))

(fn `UserConstructionScript`)